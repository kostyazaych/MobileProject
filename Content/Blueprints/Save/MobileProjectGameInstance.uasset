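; Mobile project game instance that loads the player's save slot on Init, or creates and saves a default one if loading fails.
; It caches player name, slot, user index and Virgin flag from the load node's immediate exec pin, not Completed.
; New-save defaults are likewise set after the async save starts.
; A successful load or save prints debug text, waits briefly, then fires NewEventDispatcher0.
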(event EventInit
  (bind (_savegame _bsuccess) (|AsyncLoadGamefromSlot "Slot00")
    (:then
      (bind _asmobile_project_save_game (Utilities|Casting|CastToMobileProjectSaveGame _savegame))
      (Variables|Default|SetPlayerOne (Variables|/Game/Blueprints/Save/MobileProjectSaveGame.MobileProjectSaveGame_C|GetPlayerName _asmobile_project_save_game))
      (Variables|Default|SetSlotName (Variables|/Game/Blueprints/Save/MobileProjectSaveGame.MobileProjectSaveGame_C|GetSlotName _asmobile_project_save_game))
      (Variables|Default|SetUserIndex (Variables|/Game/Blueprints/Save/MobileProjectSaveGame.MobileProjectSaveGame_C|GetUserIndex _asmobile_project_save_game))
      (Variables|Default|SetVirgin (Variables|/Game/Blueprints/Save/MobileProjectSaveGame.MobileProjectSaveGame_C|GetVirgin _asmobile_project_save_game)))
    (:Completed
      (if _bsuccess
        (Development|PrintString (Utilities|String|Append "loadSuc " (Utilities|String|ToString(Boolean) _bsuccess)) true true "(R=1.000000,G=0.000000,B=0.047066,A=1.000000)")
        (Utilities|FlowControl|Delay 2.0)
        (Default|CallNewEventDispatcher0)
        (else
          (bind _returnvalue (SaveGame|CreateSaveGameObject "/Game/Blueprints/Save/MobileProjectSaveGame.MobileProjectSaveGame_C"))
          (bind _output_get (Variables|Default|SetSaveGame _returnvalue))
          (bind _bsuccess_2 (|AsyncSaveGametoSlot _output_get "Slot00")
            (:then
              (Variables|/Game/Blueprints/Save/MobileProjectSaveGame.MobileProjectSaveGame_C|SetPlayerName (Variables|Default|GetSaveGame) "PlayerOne")
              (Variables|/Game/Blueprints/Save/MobileProjectSaveGame.MobileProjectSaveGame_C|SetVirgin (Variables|Default|GetSaveGame) true)
              (Variables|Default|SetVirgin true))
            (:Completed
              (if _bsuccess_2
                (Development|PrintString (Utilities|String|Append "SaveSuc " (Utilities|String|ToString(Boolean) _bsuccess_2)) true true "(R=1.000000,G=0.063922,B=0.000000,A=1.000000)")
                (Utilities|FlowControl|Delay 2.0)
                (Default|CallNewEventDispatcher0)))))))))